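; Shotgun projectile Blueprint whose damage to enemies falls off the longer it exists, favoring close-range hits.
; The construction script calls its parent, then sets the starting DamageDealtToEnemies.
; Tick subtracts from that value at a constant per-second rate, clamped so it stops at zero within a fraction of a second.
; This graph holds no movement or hit logic.
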(event EventBeginPlay
  (|CallParentFunction))

(event Collision|EventActorBeginOverlap
  (params (OtherActor :type Actor%20Object%20Reference))
  (|CallParentFunction 0))

(event EventTick
  (params (DeltaSeconds :type Float%20%28single-precision%29))
  (Variables|Default|SetDamageDealtToEnemies (Math|Float|Clamp(Float) (- (Variables|Default|GetDamageDealtToEnemies) (* DeltaSeconds 3e+01)) 0.0 1e+03)))

(fn ConstructionScript
  (|CallParentFunction)
  (Variables|Default|SetDamageDealtToEnemies 5.0))