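; Projectile Blueprint that damages Scuttle and Spider enemies when fired by the player, or otherwise the player, with hit sounds.
; All logic runs on actor overlap, after filtering out its firer, shield instances and a FiredBy check against PlayerCharacterTest.
; It passes through other projectiles, but shield projectiles or any non-projectile actor destroy it.
; Enemy damage uses class-specific casts and a damage variable, while player damage is hard-coded.
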(event EventBeginPlay
  (Variables|/Script/Engine.PrimitiveComponent|SetbGenerateOverlapEvents (Variables|Default|GetCollider) true))

(event EventTick
  (params (DeltaSeconds :type Float%20%28single-precision%29)))

(event Collision|EventActorBeginOverlap
  (params (OtherActor :type Actor%20Object%20Reference))
  (bind _firedby (Variables|Default|GetFiredBy))
  ;[1 1 1] Collision Logic
  (Variables|Default|SetOverlapOtherActor OtherActor)
  (if (not (== _firedby "/Game/BlueprintSource/Player/PlayerCharacterTest.PlayerCharacterTest"))
    (if (not (== _firedby (Variables|Default|GetOverlapOtherActor)))
      (if (not (Variables|Default|GetisShield))
        (bind _asprojectile_bp (Utilities|Casting|CastToProjectileBP (Variables|Default|GetOverlapOtherActor))
          (:then
            (if (Variables|ProjectileBP_C|GetisShield _asprojectile_bp)
              (Actor|DestroyActor :!label _label)
              (if (Variables|Default|GetbFiredByPlayer)
                (if (== (Utilities|GetClass (Variables|Default|GetOverlapOtherActor)) "/Game/BlueprintSource/Enemies/ScuttleEnemy.ScuttleEnemy_C")
                  (bind _asscuttle_enemy (Utilities|Casting|CastToScuttleEnemy (Variables|Default|GetOverlapOtherActor)))
                  (Default|TakeDamage _asscuttle_enemy (Variables|Default|GetDamageDealtToEnemies))
                  (Audio|PlaySound2D "/Game/Audio/SFX/EnemyDeath.EnemyDeath" 0.05 :!label _label_2)
                  (else
                    ;[1 1 1] Refactor this into enemy sometime?
                    (if (== (Utilities|GetClass (Variables|Default|GetOverlapOtherActor)) "/Game/BlueprintSource/Enemies/SpiderEnemy.SpiderEnemy_C")
                      (bind _asspider_enemy (Utilities|Casting|CastToSpiderEnemy (Variables|Default|GetOverlapOtherActor)))
                      (Default|TakeDamage _asspider_enemy (Variables|Default|GetDamageDealtToEnemies))
                      (goto _label_2))))
                (elif (== (Variables|Default|GetPlayerReference) (Variables|Default|GetOverlapOtherActor))
                  (bind _asplayer_character (Utilities|Casting|CastToPlayerCharacter (Variables|Default|GetPlayerReference)))
                  (Class|PlayerCharacter|PlayerTakeDamage _asplayer_character 14.286)
                  (Audio|PlaySound2D "/Game/Audio/SFX/CharacterHit.CharacterHit")))
              (else
                (if (not (Utilities|ClassIsChildOf (Utilities|GetClass (Variables|Default|GetOverlapOtherActor)) "ProjectileBP_C")) :!label _label_3
                  (goto _label)))))
          (:CastFailed
            (goto _label_3)))))))

(fn ConstructionScript)

(fn NewFunction0)