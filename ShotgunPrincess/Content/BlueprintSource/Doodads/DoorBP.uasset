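; Door actor that the player opens with F from inside its overlap zone, optionally requiring a matching key.
; Overlap looks up DoorName in the player's inventory, shows a HUD prompt and enables input.
; OpenDoor checks Openable, then snaps the mesh to a configured relative location, with no closing logic.
; Openable XORs the no-key and key-found cases, so holding a key for an unlocked door blocks opening.
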(event OnComponentBeginOverlap(Overlap)
  (params (OverlappedComponent :type Primitive%20Component%20Object%20Reference) (OtherActor :type Actor%20Object%20Reference) (OtherComp :type Primitive%20Component%20Object%20Reference) (OtherBodyIndex :type Integer) (bFromSweep :type Boolean) (SweepResult :type Hit%20Result%20Structure%20%28by%20ref%29))
  (if (Utilities|IsValid (Variables|Default|GetInteractor))
    _
    (else
      (bind _asplayer_character (Utilities|Casting|CastToPlayerCharacter OtherActor))
      (Variables|Default|SetInteractor _asplayer_character)))
  (Variables|Default|SetDistanceOK true)
  (Variables|/Script/ShotgunPrincess.PlayerCharacter|SetisNearDoor (Variables|Default|GetInteractor) true)
  (if (not (Variables|Default|GetisOpen))
    (bind _output_get (Variables|Default|SetKeyFound (Class|PlayerInventory|HasKey (Variables|/Script/ShotgunPrincess.PlayerCharacter|GetPlayerInventory (Variables|Default|GetInteractor)) (Variables|Default|GetDoorName))))
    (if _output_get
      (Variables|Default|SetText "Press 'F' to Open the Door" :!label _label)
      (elif (Variables|Default|GetneedsKey)
        (Variables|Default|SetText "Find the Key to this Door")
        (else
          (goto _label))))
    (Default|UITextToolTip (Variables|Default|GetHUDRef) true (Variables|Default|GetText))
    (Input|EnableInput (Variables|Default|GetControllerRef))))

(event OnComponentEndOverlap(Overlap)
  (params (OverlappedComponent :type Primitive%20Component%20Object%20Reference) (OtherActor :type Actor%20Object%20Reference) (OtherComp :type Primitive%20Component%20Object%20Reference) (OtherBodyIndex :type Integer))
  (bind _asplayer_character (Utilities|Casting|CastToPlayerCharacter OtherActor))
  (if (Utilities|IsValid _asplayer_character)
    (Variables|Default|SetDistanceOK false)
    (Variables|/Script/ShotgunPrincess.PlayerCharacter|SetisNearDoor (Variables|Default|GetInteractor) false)
    (Variables|Default|SetText "")
    (Default|UITextToolTip (Variables|Default|GetHUDRef) true (Variables|Default|GetText))
    (Input|DisableInput (Variables|Default|GetControllerRef))))

(event EventBeginPlay
  (bind _returnvalue (Game|GetPlayerController 0))
  (bind _asmain_hud (Utilities|Casting|CastToMainHUD (HUD|GetHUD _returnvalue)))
  (Variables|Default|SetHUDRef _asmain_hud)
  (Variables|Default|SetControllerRef _returnvalue))

(event EventTick
  (params (DeltaSeconds :type Float%20%28single-precision%29)))

(event Input|KeyboardEvents|F
  (params (Key :type Key%20Structure :default "AnyKey"))
  (:Pressed
    (if (Utilities|IsValid (Variables|Default|GetInteractor))
      (if (Variables|Default|GetDistanceOK)
        _
        (else
          (Variables|/Script/ShotgunPrincess.PlayerCharacter|SetisNearDoor (Variables|Default|GetInteractor) false)))
      (CallFunction|OpenDoor (Variables|Default|GetisOpen) (Variables|Default|GetXTranslate) (Variables|Default|GetYTranslate) (Variables|Default|GetZTranslate) (Variables|Default|GetInteractor)))))

(fn ConstructionScript)

(fn OpenDoor
  (params (isOpen :type Boolean) (X%20Translate :type Float%20%28single-precision%29) (Y%20Translate :type Float%20%28single-precision%29) (Z%20Translate :type Float%20%28single-precision%29) (Interactor :type Player%20Character%20Object%20Reference))
  (if (Utilities|IsValid Interactor)
    (if (not (Variables|Default|GetisOpen))
      (bind _isopenable (CallFunction|Openable Interactor))
      (if _isopenable
        (Transformation|SetRelativeLocation (Variables|Default|GetStaticMesh) (Math|Vector|MakeVector X%20Translate Y%20Translate Z%20Translate) false false)
        (Variables|Default|SetisOpen true)
        (Variables|/Script/ShotgunPrincess.PlayerCharacter|SetisOpeningDoor Interactor false)
        (Input|DisableInput (Variables|Default|GetControllerRef))))))

(fn Openable
  (params (Interactor :type Player%20Character%20Object%20Reference))
  (if (Utilities|IsValid Interactor)
    (return (Class|KismetMathLibrary|XORBoolean (and (Math|Boolean|Equal(Boolean) (Variables|Default|GetneedsKey) false) (Variables|Default|GetDistanceOK)) (and (Variables|Default|GetKeyFound) (Variables|Default|GetDistanceOK))))
    (else
      (return false))))